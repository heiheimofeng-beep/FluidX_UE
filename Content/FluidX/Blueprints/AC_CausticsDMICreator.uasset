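; Actor component that feeds BPFluidX fluid simulation data into its owner's mesh materials to show water caustics.
; On BeginPlay, a Nanite vertex check gives static meshes either a shared overlay DMI or per-slot DMIs, all fed the simulation render target, location and extent.
; Tick moves DomainCenter on per-slot DMIs to the player or fluid actor, per FollowMode.
; A note marks the overlay approach shelved because Single Layer Water hides translucency.
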(event EventBeginPlay
  (Variables|Default|GetBP_FluidX
    (:then
      (bind _returnvalue (Rendering|Material|CreateDynamicMaterialInstance "/Game/FluidX/Materials/Caustics/M_OverlayTest.M_OverlayTest" "None" "None" :!class /Script/Engine.KismetMaterialLibrary))
      (bind _output_get (Variables|Default|SetDMI_CausticsOverlay _returnvalue))
      (CallFunction|SetDMIValues _output_get)
      (for _array_element (Actor|GetComponentsByClass (Components|GetOwner) "/Script/Engine.MeshComponent")
        ;[0.7031 0.5268 0.1028 0.5] 暂时废弃，因为单层水面下不显示半透明（单层水面在半透明之前写入了深度)
        (bind _as静态网格体组件 (Utilities|Casting|CastToStaticMeshComponent _array_element)
          (:then
            (if (== (Class|StaticMesh|GetNumNaniteVertices (Variables|/Script/Engine.StaticMeshComponent|GetStaticMesh _as静态网格体组件)) -1)
              (Rendering|Material|SetOverlayMaterial _array_element (Variables|Default|GetDMI_CausticsOverlay) true 0 :!class /Script/Engine.MeshComponent)
              (else
                (for (_array_element_2 _array_index) (Rendering|Material|GetMaterials _as静态网格体组件) :!label _label
                  (bind _returnvalue_2 (Rendering|Material|CreateDynamicMaterialInstance _as静态网格体组件 _array_index _array_element_2 "None" :!class /Script/Engine.PrimitiveComponent))
                  (CallFunction|SetDMIValues _returnvalue_2)
                  (Utilities|Array|Add (Variables|Default|GetDMI_NaniteSM) _returnvalue_2)))))
          (:CastFailed
            (goto _label)))))
    (:else)))

(event EventTick
  (params (DeltaSeconds :type Float%20%28single-precision%29))
  (bind _returnvalue (Game|Player|GetPlayerPawn 0))
  (bind _bp_fluidx (Variables|Default|GetBP_FluidX))
  (bind _returnvalue_2 (Transformation|GetActorLocation _returnvalue))
  (for _array_element (Variables|Default|GetDMI_NaniteSM)
    (Rendering|Material|SetVectorParameterValue _array_element "DomainCenter" (select (Variables|/Game/FluidX/Blueprints/BP_FluidX_Water.BP_FluidX_Water_C|GetFollowMode _bp_fluidx) (Math|Conversions|ToLinearColor(Vector) (Math|Vector|MakeVector (.x _returnvalue_2) (.y _returnvalue_2) (.z _returnvalue_2))) (Math|Conversions|ToLinearColor(Vector) (Transformation|GetActorLocation _bp_fluidx))) :!class /Script/Engine.MaterialInstanceDynamic)))

(fn SetDMIValues
  (params (TargetDMI :type Material%20Instance%20Dynamic%20Object%20Reference))
  (bind _bp_fluidx (Variables|Default|GetBP_FluidX))
  (Rendering|Material|SetVectorParameterValue TargetDMI "FluidLocation" (Math|Conversions|ToLinearColor(Vector) (Transformation|GetActorLocation _bp_fluidx)) :!class /Script/Engine.MaterialInstanceDynamic)
  (Rendering|Material|SetVectorParameterValue TargetDMI "WorldExtent" (Math|Conversions|ToLinearColor(Vector) (* (Transformation|GetActorScale3D _bp_fluidx) "1000.000000,1000.000000,64.000000")) :!class /Script/Engine.MaterialInstanceDynamic)
  (Rendering|Material|SetTextureParameterValue TargetDMI "SimRT" (Variables|/Game/FluidX/Blueprints/BP_FluidX_Water.BP_FluidX_Water_C|GetRT_Fluid _bp_fluidx))
  (Rendering|Material|SetScalarParameterValue TargetDMI "UseCaustics" 1.0 :!class /Script/Engine.MaterialInstanceDynamic)
  (Rendering|Material|SetScalarParameterValue TargetDMI "WorldExtent" (.x (Variables|/Game/FluidX/Blueprints/BP_FluidX_Water.BP_FluidX_Water_C|GetWorldExtent (Variables|Default|GetBP_FluidX))) :!class /Script/Engine.MaterialInstanceDynamic))