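; BP_FluidX_Water is an interactive water surface driven by a Niagara fluid simulation.
; The construction script links the simulation to the water material through a runtime render target.
; Point damage and moving overlapping actors with AC_FluidInteractionSettings queue splashes into Niagara arrays, cleared the next frame.
; In follow mode, the simulation domain scrolls with the player pawn on XY, passing its shift to Niagara and its center to both.
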(event Custom|SpawnSplash
  (params (InValue :type Vector) (SplashRadius :type Float%20%28double-precision%29) (SplashStrength :type Float%20%28double-precision%29) (HitVelocity :type Float%20%28double-precision%29) (HitObjectVelocities :type Vector))
  (bind _niagarafx (Variables|Default|GetNiagaraFX))
  ;[0.15 0.15 0.15 0.5 50] 产生水花
  (Utilities|Array|Add (Variables|Default|GetCurrentHitPositions) InValue)
  (Utilities|Array|Add (Variables|Default|GetSplashRadii) (* SplashRadius 1.0))
  (Utilities|Array|Add (Variables|Default|GetSplashStrengths) (* SplashStrength 0.1))
  (Utilities|Array|Add (Variables|Default|GetHitVelocities) (* HitVelocity 1.0))
  (Utilities|Array|Add (Variables|Default|GetHitObjectVelocities) (* HitObjectVelocities 1.0))
  (Class|NiagaraDataInterfaceArrayFunctionLibrary|SetNiagaraArrayFloat _niagarafx "SplashRadii" (Variables|Default|GetSplashRadii))
  (Class|NiagaraDataInterfaceArrayFunctionLibrary|SetNiagaraArrayFloat _niagarafx "SplashStrengths" (Variables|Default|GetSplashStrengths))
  (Class|NiagaraDataInterfaceArrayFunctionLibrary|SetNiagaraArrayFloat _niagarafx "HitVelocities" (Variables|Default|GetHitVelocities))
  (Class|NiagaraComponent|SetVariableInt (Variables|Default|GetNiagaraFX) "HitCount" (Utilities|Array|Length (Variables|Default|GetCurrentHitPositions)))
  (Class|NiagaraDataInterfaceArrayFunctionLibrary|SetNiagaraArrayVector (Variables|Default|GetNiagaraFX) "HitPositions" (Variables|Default|GetCurrentHitPositions))
  (Class|NiagaraDataInterfaceArrayFunctionLibrary|SetNiagaraArrayVector (Variables|Default|GetNiagaraFX) "HitObjectVelocities" (Variables|Default|GetHitObjectVelocities))
  (Utilities|FlowControl|DelayUntilNextFrame)
  (CallFunction|ResetHitPositions))

(event EventBeginPlay)

(event Collision|EventActorBeginOverlap
  (params (OtherActor :type Actor%20Object%20Reference)))

(event Game|Damage|EventPointDamage
  (params (Damage :type Float%20%28single-precision%29) (DamageType :type Damage%20Type%20Object%20Reference) (HitLocation :type Vector :default "0, 0, 0") (HitNormal :type Vector :default "0, 0, 0") (HitComponent :type Primitive%20Component%20Object%20Reference) (BoneName :type Name :default "None") (ShotFromDirection :type Vector :default "0, 0, 0") (InstigatedBy :type Controller%20Object%20Reference) (DamageCauser :type Actor%20Object%20Reference) (HitInfo :type Hit%20Result%20Structure%20%28by%20ref%29))
  (CallFunction|SpawnSplash HitLocation (Math|Float|MapRangeClamped Damage 0.0 5e+02 0.0 5e+02) (Math|Float|MapRangeClamped Damage 0.0 1e+02 0.0 1e+02) (Math|Float|MapRangeClamped Damage 0.0 5e+02 0.0 1e+04) (* (* ShotFromDirection -1) (Math|Float|MapRangeClamped Damage 0.0 5e+02 0.0 1e+04))))

(event Game|Damage|EventRadialDamage
  (params (DamageReceived :type Float%20%28single-precision%29) (DamageType :type Damage%20Type%20Object%20Reference) (Origin :type Vector :default "0, 0, 0") (HitInfo :type Hit%20Result%20Structure%20%28by%20ref%29) (InstigatedBy :type Controller%20Object%20Reference) (DamageCauser :type Actor%20Object%20Reference)))

(event EventTick
  (params (DeltaSeconds :type Float%20%28single-precision%29))
  (Utilities|FlowControl|Sequence
    (:then_0
      (CallFunction|UpdateActorSplash))
    (:then_1
      (if (Variables|Default|GetFollowMode)
        (CallFunction|UpdateDomainScroll)
        (else
          (Rendering|Material|SetVectorParameterValue (Variables|Default|GetDMI_Fluid) "DomainCenter" (Math|Conversions|ToLinearColor(Vector) (Transformation|GetActorLocation)) :!class /Script/Engine.MaterialInstanceDynamic))))))

(fn ConstructionScript
  (bind _niagarafx (Variables|Default|GetNiagaraFX))
  (Utilities|FlowControl|Sequence
    (:then_0
      (if (Variables|Default|GetUseBoxExtent)
        (Variables|Default|SetWorldExtent (* (Components|Box|GetScaledBoxExtent (Variables|Default|GetBox)) 2))))
    (:then_1
      (Class|NiagaraComponent|SetAsset (Variables|Default|GetNiagaraFX) (Variables|Default|GetNS_Fluid) true)
      (bind _returnvalue (Rendering|Material|CreateDynamicMaterialInstance (Variables|Default|GetWaterMesh) 0 (Variables|Default|GetWaterMaterial) "None" :!class /Script/Engine.PrimitiveComponent))
      (bind _output_get (Variables|Default|SetDMI_Fluid _returnvalue))
      (Rendering|Material|SetMaterial (Variables|Default|GetWaterMesh) 0 _output_get)
      (Niagara|SetNiagaraVariable(Vector3) _niagarafx "WorldExtent" (Variables|Default|GetWorldExtent))
      (Class|NiagaraComponent|SetVariableInt _niagarafx "Resolution" (Variables|Default|GetResolution))
      (bind _returnvalue_2 (Rendering|CreateRenderTarget2D 512 512 "RTF_RGBA16f"))
      (Variables|Default|SetRT_Fluid _returnvalue_2)
      (Class|NiagaraComponent|SetVariableTextureRenderTarget (Variables|Default|GetNiagaraFX) "SimRT" (Variables|Default|GetRT_Fluid))
      (Rendering|Material|SetTextureParameterValue (Variables|Default|GetDMI_Fluid) "SimRT" (Variables|Default|GetRT_Fluid))
      (Rendering|Material|SetScalarParameterValue (Variables|Default|GetDMI_Fluid) "WorldExtent" (.x (Variables|Default|GetWorldExtent)) :!class /Script/Engine.MaterialInstanceDynamic))
    (:then_2
      (Niagara|SetNiagaraVariable(Float) (Variables|Default|GetNiagaraFX) "FollowBlend" (Math|Conversions|ToFloat(Boolean) (Variables|Default|GetFollowMode)))
      (Class|NiagaraComponent|SetVariableInt (Variables|Default|GetNiagaraFX) "BoundaryMode" (Math|Conversions|ToInteger(Byte) (Variables|Default|GetBoundaryMode))))))

(fn ResetHitPositions
  (bind _niagarafx (Variables|Default|GetNiagaraFX))
  (bind _currenthitpositions (Variables|Default|GetCurrentHitPositions))
  (bind _niagarafx_2 (Variables|Default|GetNiagaraFX))
  (Variables|Default|SetPrevHit%20Positions _currenthitpositions)
  (Utilities|Array|Clear _currenthitpositions)
  (Utilities|Array|Clear (Variables|Default|GetSplashRadii))
  (Utilities|Array|Clear (Variables|Default|GetSplashStrengths))
  (Utilities|Array|Clear (Variables|Default|GetHitVelocities))
  (Utilities|Array|Clear (Variables|Default|GetHitObjectVelocities))
  (Class|NiagaraDataInterfaceArrayFunctionLibrary|SetNiagaraArrayVector _niagarafx_2 "HitPositions" (Variables|Default|GetCurrentHitPositions))
  (Class|NiagaraDataInterfaceArrayFunctionLibrary|SetNiagaraArrayVector _niagarafx_2 "PrevHitPositions" (Variables|Default|GetPrevHit%20Positions))
  (Class|NiagaraComponent|SetVariableInt _niagarafx_2 "HitCount")
  (Class|NiagaraDataInterfaceArrayFunctionLibrary|SetNiagaraArrayFloat _niagarafx "SplashRadii" (Variables|Default|GetSplashRadii))
  (Class|NiagaraDataInterfaceArrayFunctionLibrary|SetNiagaraArrayFloat _niagarafx "SplashStrengths" (Variables|Default|GetSplashStrengths))
  (Class|NiagaraDataInterfaceArrayFunctionLibrary|SetNiagaraArrayFloat _niagarafx "HitVelocities" (Variables|Default|GetHitVelocities))
  (Class|NiagaraDataInterfaceArrayFunctionLibrary|SetNiagaraArrayVector (Variables|Default|GetNiagaraFX) "HitObjectVelocities" (Variables|Default|GetHitObjectVelocities)))

(fn UpdateOverlapActorSplash
  (params (Velocity :type Vector) (Location :type Vector))
  (bind _returnvalue (Math|Vector|VectorLength Velocity))
  (if (> _returnvalue 15.0)
    (bind _hitlocation (Collision|LineTraceComponent (Variables|Default|GetWaterMesh) (+ Location "0.000000,0.000000,155.000000") (- Location "0.000000,0.000000,555.000000") true false false))
    (CallFunction|SpawnSplash _hitlocation 25.0 (Math|Float|MapRangeClamped _returnvalue 15.0 1e+03 5.0 5e+01) (Math|Float|MapRangeClamped _returnvalue 15.0 1e+03 1e+02 1e+03) Velocity)
    (if (Variables|Default|GetDebug)
      (Rendering|Debug|DrawDebugSphere _hitlocation 55.0 12 "(R=1.000000,G=0.545677,B=0.000000,A=1.000000)" (Class|Actor|GetActorTickInterval) 1.0))))

(fn UpdateActorSplash
  (bind _watermesh (Variables|Default|GetWaterMesh))
  (bind _overlappingactors (Collision|GetOverlappingActors _watermesh "/Script/Engine.Actor" :!class /Script/Engine.PrimitiveComponent))
  (if (not (Utilities|Array|IsEmpty _overlappingactors))
    (for _array_element _overlappingactors
      (Utilities|IsValid (Actor|GetComponentbyClass _array_element "/Game/FluidX/Blueprints/AC_FluidInteractionSettings.AC_FluidInteractionSettings_C")
        (:Is%20Valid
          (bind (_velocity _locations) (Default|GetInteractionSettings (Actor|GetComponentbyClass _array_element "/Game/FluidX/Blueprints/AC_FluidInteractionSettings.AC_FluidInteractionSettings_C")))
          (for (_array_element_2 _array_index) _velocity
            (CallFunction|UpdateOverlapActorSplash _array_element_2 (Utilities|Array|Get(acopy) _locations _array_index))))))))

(fn UpdateDomainScroll
  (bind _returnvalue (Game|Player|GetPlayerPawn 0))
  (bind _returnvalue_2 (Transformation|GetActorLocation))
  (bind _returnvalue_3 (Transformation|GetActorLocation _returnvalue))
  (bind _returnvalue_4 (Math|Vector|MakeVector (.x _returnvalue_3) (.y _returnvalue_3) (.z _returnvalue_2)))
  (Niagara|SetNiagaraVariable(Vector3) (Variables|Default|GetNiagaraFX) "DomainCenter" _returnvalue_4)
  (Niagara|SetNiagaraVariable(Vector3) (Variables|Default|GetNiagaraFX) "DomainShiftWorld" (- _returnvalue_4 (Variables|Default|GetPrevDomainCenter)))
  (Rendering|Material|SetVectorParameterValue (Variables|Default|GetDMI_Fluid) "DomainCenter" (Math|Conversions|ToLinearColor(Vector) _returnvalue_4) :!class /Script/Engine.MaterialInstanceDynamic)
  (Variables|Default|SetPrevDomainCenter (Transformation|GetActorLocation (Game|Player|GetPlayerPawn 0))))