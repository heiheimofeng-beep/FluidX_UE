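; Actor component that supplies velocity and location data from its owner, apparently for FluidX fluid interaction.
; On BeginPlay it finds the owner's primitive component whose object name matches ComponentName.
; GetInteractionSettings returns physics linear velocities and world locations for each listed socket, or for the component itself when no sockets are set.
; Socket results are gathered with AddUnique, so duplicate values collapse independently in each array.
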(event EventBeginPlay
  (for _array_element (Actor|GetComponentsByClass (Components|GetOwner) "/Script/Engine.PrimitiveComponent")
    (if (Utilities|Enum|Equal(Enum) (Utilities|GetObjectName _array_element) (Utilities|String|ToString(Name) (Variables|Default|GetComponentName)))
      (Variables|Default|SetTargetComponent _array_element))))

(event EventTick
  (params (DeltaSeconds :type Float%20%28single-precision%29)))

(fn GetInteractionSettings
  (if (Utilities|Array|IsNotEmpty (Variables|Default|GetSockets))
    (for _array_element (Variables|Default|GetSockets)
      (bind _returnvalue (Physics|GetPhysicsLinearVelocity (Variables|Default|GetTargetComponent) _array_element))
      (Utilities|Array|AddUnique (LocalVariables|GetSocketVelocity) _returnvalue)
      (Utilities|Array|AddUnique (LocalVariables|GetSocketLocations) (Transformation|GetSocketLocation (Variables|Default|GetTargetComponent) _array_element)))
    (return (LocalVariables|GetSocketVelocity) (LocalVariables|GetSocketLocations))
    (else
      (bind _returnvalue_2 (Physics|GetPhysicsLinearVelocity (Variables|Default|GetTargetComponent) "None"))
      (return (Utilities|Array|MakeArray _returnvalue_2) (Utilities|Array|MakeArray (Transformation|GetWorldLocation (Variables|Default|GetTargetComponent)))))))